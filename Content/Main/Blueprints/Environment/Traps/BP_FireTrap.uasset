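; BP_FireTrap is an environmental trap that damages the player with fire while they stand in its Box.
; Box overlap begin and end show or hide the particle system after short delays, for the player only.
; Tick re-fetches the player character and, while particles are visible and the player overlaps, removes a heart and checks death.
; A DoOnce reset after a delay turns this into damage repeated at one-second intervals.
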(event OnComponentBeginOverlap(Box)
  (params (OverlappedComponent :type Primitive%20Component%20Object%20Reference) (OtherActor :type Actor%20Object%20Reference) (OtherComp :type Primitive%20Component%20Object%20Reference) (OtherBodyIndex :type Integer) (bFromSweep :type Boolean) (SweepResult :type Hit%20Result%20Structure%20%28by%20ref%29))
  ;[0.15 0.15 0.15 0.5] box와 플레이어가 오버랩 되면 딜레이 후 파티클이 보임
  (if (== OtherActor (Variables|Default|GetPlayer%20Ref))
    (Utilities|FlowControl|Delay 0.3)
    (Rendering|SetVisibility (Variables|Default|GetParticleSystem) true false)))

(event OnComponentEndOverlap(Box)
  (params (OverlappedComponent :type Primitive%20Component%20Object%20Reference) (OtherActor :type Actor%20Object%20Reference) (OtherComp :type Primitive%20Component%20Object%20Reference) (OtherBodyIndex :type Integer))
  ;[0.15 0.15 0.15 0.5] box와 플레이어 오버랩이 끝나면 딜레이 후 파티클 사라짐
  (if (== OtherActor (Variables|Default|GetPlayer%20Ref))
    (Utilities|FlowControl|Delay 1.0)
    (Rendering|SetVisibility (Variables|Default|GetParticleSystem) false false)))

(event EventBeginPlay
  (CallFunction|RetrackPlayer))

(event EventTick
  (params (DeltaSeconds :type Float%20%28single-precision%29))
  (bind _player_ref (Variables|Default|GetPlayer%20Ref))
  ;[0.15 0.15 0.15 0.5] 파티클이 보일 때 박스와 오버랩되면 데미지 1. 박스에서 벗어나지 않으면 1초 간격으로 도트 데미지
  (CallFunction|RetrackPlayer)
  (if (Rendering|IsVisible (Variables|Default|GetParticleSystem))
    (if (Collision|IsOverlappingActor (Variables|Default|GetBox) (Variables|Default|GetPlayer%20Ref) :!class /Script/Engine.PrimitiveComponent)
      (Utilities|FlowControl|DoOnce false :!label _label
        (:Completed
          (Default|LoseHeart _player_ref 1)
          (Default|CheckDeath _player_ref)
          (Utilities|FlowControl|Delay 1.0)
          (goto _label Reset))))))

(fn ConstructionScript)

(fn RetrackPlayer
  (bind _asbp_player_character_base (Utilities|Casting|CastToBP_PlayerCharacterBase (Game|GetPlayerCharacter 0)))
  (Variables|Default|SetPlayer%20Ref _asbp_player_character_base))