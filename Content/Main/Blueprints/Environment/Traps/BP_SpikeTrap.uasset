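; BP_SpikeTrap is a spike trap that damages the player while they stand inside its box.
; BeginPlay caches player 0 as a BP_PlayerCharacterBase reference.
; Every Tick checks whether the box overlaps that player, removes one heart and runs the death check.
; A DoOnce reset after a one-second delay turns continued overlap into once-per-second damage instead of using overlap events.
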(event EventBeginPlay
  (bind _asbp_player_character_base (Utilities|Casting|CastToBP_PlayerCharacterBase (Game|GetPlayerCharacter 0)))
  (Variables|Default|SetPlayer%20Ref _asbp_player_character_base))

(event EventTick
  (params (DeltaSeconds :type Float%20%28single-precision%29))
  (bind _player_ref (Variables|Default|GetPlayer%20Ref))
  ;[0.15 0.15 0.15 0.5] 박스와 오버랩되면 데미지 1. 박스에서 벗어나지 않으면 1초 간격으로 도트 데미지
  (if (Collision|IsOverlappingActor (Variables|Default|GetBox) (Variables|Default|GetPlayer%20Ref) :!class /Script/Engine.PrimitiveComponent)
    (Utilities|FlowControl|DoOnce false :!label _label
      (:Completed
        (Default|LoseHeart _player_ref 1)
        (Default|CheckDeath _player_ref)
        (Utilities|FlowControl|Delay 1.0)
        (goto _label Reset)))))

(fn ConstructionScript)