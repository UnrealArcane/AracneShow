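; Fire trap actor that plays a growing Niagara fire effect and takes hearts from the player standing inside its box.
; On BeginPlay it caches the player, plays a 2D fire sound and runs a timeline driving the Niagara Progress parameter, with GrowSpeed setting the play rate.
; Tick polls box overlap, using a DoOnce reset after a delay to remove a heart and check death about once per second.
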(event EventBeginPlay
  (bind _asbp_player_character_base (Utilities|Casting|CastToBP_PlayerCharacterBase (Game|GetPlayerCharacter 0)))
  (Variables|Default|SetPlayer%20Ref _asbp_player_character_base)
  (Audio|PlaySound2D "/Game/ThirdParty/StarterContent/Audio/Fire01_Cue.Fire01_Cue" 1.0 1.0 0.0 0 0)
  (bind _newtrack_0 (Timeline|Timeline Play)
    (:Update
      (Niagara|SetNiagaraVariable(Float) (Variables|Default|GetNiagara) "Progress" _newtrack_0))))

(event Collision|EventActorBeginOverlap
  (params (OtherActor :type Actor%20Object%20Reference)))

(event EventTick
  (params (DeltaSeconds :type Float%20%28single-precision%29))
  (bind _player_ref (Variables|Default|GetPlayer%20Ref))
  ;[0.15 0.15 0.15 0.5] 박스에서 벗어나지 않으면 1초 간격으로 도트 데미지
  (if (Collision|IsOverlappingActor (Variables|Default|GetBox) (Variables|Default|GetPlayer%20Ref) :!class /Script/Engine.PrimitiveComponent)
    (Utilities|FlowControl|DoOnce false :!label _label
      (:Completed
        (Default|LoseHeart _player_ref 1)
        (Default|CheckDeath _player_ref)
        (Utilities|FlowControl|Delay 1.0)
        (goto _label Reset)))))

(fn ConstructionScript
  (Components|Timeline|SetPlayRate (Variables|Default|GetTimeline) (Variables|Default|GetGrowSpeed)))