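; BP_CoinCollectible is a spinning coin pickup that adds one to a coin count when overlapped.
; Tick rotates CoinMesh around yaw by CoinSpinRate each frame, without delta-time scaling.
; Any overlap with PickupCollision increments Coins on the DA reference, destroys the coin, prints the total and plays a 2D collect sound.
; An unconnected branch that would credit the instigator's BP_PosseasbleCharacter instead never runs.
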(event OnComponentBeginOverlap(PickupCollision)
  (params (OverlappedComponent :type Primitive%20Component%20Object%20Reference) (OtherActor :type Actor%20Object%20Reference) (OtherComp :type Primitive%20Component%20Object%20Reference) (OtherBodyIndex :type Integer) (bFromSweep :type Boolean) (SweepResult :type Hit%20Result%20Structure%20%28by%20ref%29))
  (bind _da (Variables|Default|GetDA))
  (bind _coins (Variables|/Game/Main/Blueprints/DataAsset/PDA_CharacterInformation.PDA_CharacterInformation_C|GetCoins _da))
  (Math|Integer|IncrementInt _coins
    (:%20%20
      (Actor|DestroyActor)
      (Development|PrintString (Utilities|String|ToString(Integer) _coins))
      (Audio|PlaySound2D "/Game/Main/Audio/Collect_Point_01.Collect_Point_01" 1.0 1.0 0.0 0 0))))

(event EventTick
  (params (DeltaSeconds :type Float%20%28single-precision%29))
  (Transformation|AddRelativeRotation (Variables|Default|GetCoinMesh) (Math|Rotator|MakeRotator 0.0 0.0 (Variables|Default|GetCoinSpinRate)) false false))

(fn ConstructionScript)