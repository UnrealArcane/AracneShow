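; Default player character Blueprint that throws possession cards and serves as the un-possessed base state.
; The attack input spawns a BP_PossessCards actor just ahead of the character with itself as instigator, then destroys it after a short delay if still valid.
; The cancel-possess input calls an empty placeholder function, so cancelling possession does nothing in this default state.
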(event Input|EnhancedActionEvents|EnhancedInputActionIA_Attack
  (params (ActionValue :type Boolean) (ElapsedSeconds :type Float%20%28double-precision%29) (TriggeredSeconds :type Float%20%28double-precision%29) (InputAction :type Input%20Action%20Object%20Reference :default "/Game/Main/Input/Actions/IA_Attack.IA_Attack"))
  (bind _returnvalue (Transformation|GetActorTransform))
  ;[0.15 0.15 0.15 0.5] Attack 키가 눌렸을 때 Card 발사
  (:Started
    (bind _returnvalue_2 (Game|SpawnActorfromClass "/Game/Main/Blueprints/Abilities/BP_PossessCards.BP_PossessCards_C" (Math|Transform|MakeTransform (+ (.location _returnvalue) (* (Transformation|GetActorForwardVector) 1e+02)) (.rotation _returnvalue) "1.000000,1.000000,1.000000") "Undefined" "MultiplyWithRoot" 0 self))
    (Utilities|FlowControl|Delay 0.7)
    (Utilities|IsValid _returnvalue_2
      (:Is%20Valid
        (Actor|DestroyActor _returnvalue_2)))))

(event Input|EnhancedActionEvents|EnhancedInputActionIA_CancelPosses
  (params (ActionValue :type Boolean) (ElapsedSeconds :type Float%20%28double-precision%29) (TriggeredSeconds :type Float%20%28double-precision%29) (InputAction :type Input%20Action%20Object%20Reference :default "/Game/Main/Input/Actions/IA_CancelPosses.IA_CancelPosses"))
  ;[0.15 0.15 0.15 0.5] 기본 캐릭터 상태일 때 빙의 취소 방지
  (:Started
    (CallFunction|NewFunction0)))

(fn ConstructionScript
  (|CallParentFunction))

(fn NewFunction0)