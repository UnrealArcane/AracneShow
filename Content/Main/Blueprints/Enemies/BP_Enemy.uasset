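; BP_Enemy is an enemy that drains the player's hearts on contact.
; It caches player 0 as a BP_PlayerCharacterBase on BeginPlay and again on any actor overlap.
; Tick polls whether the Capsule overlaps that player, then removes one heart and runs the player's death check.
; A DoOnce reset after a one-second delay limits how often damage repeats during continuous contact.
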(event EventBeginPlay
  (bind _asbp_player_character_base (Utilities|Casting|CastToBP_PlayerCharacterBase (Game|GetPlayerCharacter 0)))
  (Variables|Default|SetPlayer%20Ref _asbp_player_character_base))

(event Collision|EventActorBeginOverlap
  (params (OtherActor :type Actor%20Object%20Reference))
  (bind _asbp_player_character_base (Utilities|Casting|CastToBP_PlayerCharacterBase (Game|GetPlayerCharacter 0)))
  (Variables|Default|SetPlayer%20Ref _asbp_player_character_base))

(event EventTick
  (params (DeltaSeconds :type Float%20%28single-precision%29))
  (bind _player_ref (Variables|Default|GetPlayer%20Ref))
  ;[0.15 0.15 0.15 0.5] Damage
  (if (Collision|IsOverlappingActor (Variables|Default|GetCapsule) (Variables|Default|GetPlayer%20Ref) :!class /Script/Engine.PrimitiveComponent)
    (Utilities|FlowControl|DoOnce false :!label _label
      (:Completed
        (Default|LoseHeart _player_ref 1)
        (Default|CheckDeath _player_ref)
        (Utilities|FlowControl|Delay 1.0)
        (goto _label Reset)))))

(fn ConstructionScript)