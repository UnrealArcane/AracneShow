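; BP_Spikes is a spike trap that deals damage over time to a BP_PosseasbleCharacter inside its Box.
; Begin overlap casts the overlapping actor's Instigator, sets IsInTrap, then removes one heart and checks for death immediately.
; A Delay loop repeats the damage every DOTTickRate while IsInTrap stays true.
; End overlap clears that single flag, which is shared by all overlapping characters.
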(event OnComponentBeginOverlap(Box)
  (params (OverlappedComponent :type Primitive%20Component%20Object%20Reference) (OtherActor :type Actor%20Object%20Reference) (OtherComp :type Primitive%20Component%20Object%20Reference) (OtherBodyIndex :type Integer) (bFromSweep :type Boolean) (SweepResult :type Hit%20Result%20Structure%20%28by%20ref%29))
  (bind _asbp_posseasble_character (Utilities|Casting|CastToBP_PosseasbleCharacter (Game|GetInstigator OtherActor)))
  (Variables|Default|SetIsInTrap true)
  (Default|LoseHeart _asbp_posseasble_character 1 :!label _label)
  (Default|CheckDeath _asbp_posseasble_character)
  (Utilities|FlowControl|Delay (Variables|Default|GetDOTTickRate))
  (if (Variables|Default|GetIsInTrap)
    (goto _label)))

(event OnComponentEndOverlap(Box)
  (params (OverlappedComponent :type Primitive%20Component%20Object%20Reference) (OtherActor :type Actor%20Object%20Reference) (OtherComp :type Primitive%20Component%20Object%20Reference) (OtherBodyIndex :type Integer))
  (Utilities|Casting|CastToBP_PosseasbleCharacter (Game|GetInstigator OtherActor))
  (Variables|Default|SetIsInTrap false))

(event EventBeginPlay)

(event Collision|EventActorBeginOverlap
  (params (OtherActor :type Actor%20Object%20Reference)))

(event EventTick
  (params (DeltaSeconds :type Float%20%28single-precision%29)))

(fn ConstructionScript)