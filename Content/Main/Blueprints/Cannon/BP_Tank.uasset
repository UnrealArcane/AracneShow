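; BP_Tank is a tank Blueprint that fires its cannon when the IA_Fire Enhanced Input action starts.
; The FIre function plays a montage on the mesh and immediately skips to a fixed position within it.
; It then spawns an explosion emitter and an actor, whose class is not shown, at the Arrow1 component, and plays a non-spatial 2D explosion sound.
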(event Input|EnhancedActionEvents|EnhancedInputActionIA_Fire
  (params (ActionValue :type Boolean) (ElapsedSeconds :type Float%20%28double-precision%29) (TriggeredSeconds :type Float%20%28double-precision%29) (InputAction :type Input%20Action%20Object%20Reference :default "/Game/Main/Blueprints/Cannon/IA_Fire.IA_Fire"))
  (:Started
    (CallFunction|FIre)))

(event EventBeginPlay)

(event Collision|EventActorBeginOverlap
  (params (OtherActor :type Actor%20Object%20Reference)))

(event EventTick
  (params (DeltaSeconds :type Float%20%28single-precision%29)))

(fn ConstructionScript)

(fn FIre
  (Animation|Montage|MontagePlay (Components|SkeletalMesh|GetAnimInstance (Variables|Character|GetMesh)) "/Game/ThirdParty/simple-cannon/source/Simple_Cannon/model/FBX/TankMontage2.TankMontage2" 1.0 "MontageLength" 0.0 true)
  (Class|AnimInstance|MontageSetPosition (Components|SkeletalMesh|GetAnimInstance (Variables|Character|GetMesh)) "/Game/ThirdParty/simple-cannon/source/Simple_Cannon/model/FBX/TankMontage2.TankMontage2" 4.48)
  (Effects|SpawnEmitteratLocation "/Game/ThirdParty/StarterContent/Particles/P_Explosion.P_Explosion" (Transformation|GetWorldLocation (Variables|Default|GetArrow1)))
  (Game|SpawnActorfromClass "/Game/Main/Blueprints/Cannon/BP_Bullet.BP_Bullet_C" (Transformation|GetWorldTransform (Variables|Default|GetArrow1)) "Undefined" "MultiplyWithRoot" 0 0)
  (Audio|PlaySound2D "/Game/ThirdParty/StarterContent/Audio/Explosion02.Explosion02" 1.0 1.0 0.0 0 0))