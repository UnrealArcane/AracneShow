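; BP_Dragon is a dragon character Blueprint that adds player-controlled flight.
; Pressing Fly switches CharacterMovement to Flying, sets IsFly and plays a flapping sound; releasing it switches to Falling and clears the flag.
; The Fly axis adds movement input along the up vector of a yaw-only control rotation, so the dragon climbs straight up.
; Landing also clears IsFly.
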(event EventBeginPlay)

(event Collision|EventActorBeginOverlap
  (params (OtherActor :type Actor%20Object%20Reference)))

(event EventOnLanded
  (params (Hit :type Hit%20Result%20Structure%20%28by%20ref%29))
  ;[0.15 0.15 0.15 0.5] 땅에 닿았는지 판단
  (Variables|Default|SetIsFly false))

(event EventTick
  (params (DeltaSeconds :type Float%20%28single-precision%29)))

(event Input|ActionEvents|InputActionFly
  (params (Key :type Key%20Structure :default "None"))
  (bind _charactermovement (Variables|Character|GetCharacterMovement))
  ;[0.15 0.15 0.15 0.5] Fly
  (:Pressed
    (Pawn|Components|CharacterMovement|SetMovementMode _charactermovement "MOVE_Flying" 0)
    (Variables|Default|SetIsFly true)
    (Audio|PlaySound2D "/Game/ThirdParty/sound/flapping-39306.flapping-39306" 1.0 1.0 0.0 0 0))
  (:Released
    (Pawn|Components|CharacterMovement|SetMovementMode _charactermovement "MOVE_Falling" 0)
    (Variables|Default|SetIsFly false)))

(event Input|AxisEvents|InputAxisFly
  (params (AxisValue :type Float%20%28single-precision%29))
  ;[0.15 0.15 0.15 0.5] fly 진행 시 하늘 위로 오르도록 조정
  (Pawn|Input|AddMovementInput (Math|Vector|GetUpVector (Math|Rotator|MakeRotator 0.0 0.0 (.yaw (Pawn|GetControlRotation :!class /Script/Engine.Pawn)))) AxisValue false))

(fn ConstructionScript)